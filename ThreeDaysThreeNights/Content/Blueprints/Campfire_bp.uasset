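; Campfire that burns down fuel over time and loses the game if it stays out too long.
; Each tick until the game is lost, fuel drives point light intensity on a squared curve, Niagara fire strength linearly, and linked dimming fires' strength.
; The world light stays at full brightness while any fuel remains, otherwise zero.
; AddFuel refuels it; at zero fuel a dark timer counts down to the game mode's Lose, resetting when fuel returns.
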(event Custom|Add%20Fuel
  (params (Fuel :type Float%20%28double-precision%29))
  (Variables|Burning|SetFuel (Math|Float|Clamp(Float) (+ Fuel (Variables|Burning|GetFuel)) 0.0 (Variables|Burning|GetMax%20Fuel))))

(event EventTick
  (params (DeltaSeconds :type Float%20%28single-precision%29))
  (bind _max_fuel (Variables|Burning|GetMax%20Fuel))
  (bind _as3d3n_gm (Utilities|Casting|CastTo3D3N_gm (Game|GetGameMode)))
  (if (not (Variables|/Game/Blueprints/3D3N_gm.3D3N_gm_C|GetLost _as3d3n_gm))
    (Utilities|FlowControl|Sequence
      (:then_0
        (bind _output_get (Variables|Burning|SetFuel (Math|Float|Clamp(Float) (- (Variables|Burning|GetFuel) (* (Variables|Burning|GetBurn%20Rate) DeltaSeconds)) 0.0 _max_fuel)))
        (Rendering|Components|Light|SetIntensity (Variables|Default|GetPointLight) (Math|Float|Lerp 0.0 (Variables|Burning|GetMax%20Light%20Intensity) (* (/ _output_get _max_fuel) (/ _output_get _max_fuel))))
        (Effects|Components|ParticleSystem|SetFloatParameter (Variables|Default|GetNiagara) "Fire Strength" (Math|Float|Lerp 0.0 (Variables|Burning|GetMax%20Fire%20Strength) (/ _output_get _max_fuel)))
        (bind _result (Utilities|Set|ToArray (Variables|Burning|GetDimming%20Fires)))
        (for _array_element _result
          (Utilities|IsValid _array_element
            (:Is%20Valid
              (Variables|/Game/Blueprints/Fire_bp.Fire_bp_C|SetStrength _array_element (/ _output_get _max_fuel)))))
        (bind _world_light (Variables|Burning|GetWorld%20Light)
          (:then
            (Rendering|Components|Light|SetIntensity (Variables|/Script/Engine.Light|GetLightComponent _world_light) (Math|Float|Lerp 0.0 (Variables|Burning|GetWorld%20Light%20Maximum%20Brightness) (Math|Float|SelectFloat (/ (/ _output_get _max_fuel) (/ _output_get _max_fuel)) 0.0 (> (/ _output_get _max_fuel) 0.0)))))
          (:else)))
      (:then_1
        (if (<= (Variables|Burning|GetFuel) 0.0)
          (bind _output_get_2 (Variables|Default|SetDark%20Timer (- (Variables|Default|GetDark%20Timer) DeltaSeconds)))
          (if (<= _output_get_2 0.0)
            (bind _as3d3n_gm_2 (Utilities|Casting|CastTo3D3N_gm (Game|GetGameMode)))
            (Default|Lose _as3d3n_gm_2 "\"And for fear of him the keepers did shake, and became as dead men.\" - Matthew 28:4 KJV" "The Fire Was Out Too Long" "Make sure to keep the fire burning! Your assistant can gather wood for you if you send them into the forest." "/Game/Audio/Sounds/Fire_Out.Fire_Out"))
          (else
            (Variables|Default|SetDark%20Timer (Variables|Default|GetDark%20Time))))))))

(fn ConstructionScript)