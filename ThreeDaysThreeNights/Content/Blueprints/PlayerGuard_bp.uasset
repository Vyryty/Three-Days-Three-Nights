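; PlayerGuard is a first-person guard player Blueprint that adds the GUI widget on BeginPlay and can turn its camera around to look behind.
; TurnAround plays or reverses the Turn timeline based on the Backwards state, lerping the camera from its construction-time forward rotation and flipping that state when finished.
; Yaw offsets just either side of 180 degrees let the shortest-path lerp pick the turn direction.
; Construction also fills Stamina to its maximum.
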(event Custom|Turn%20Around
  (params (Left :type Boolean))
  (bind _forward_rotation (Variables|Turning|GetForward%20Rotation))
  (bind (_roll _pitch _yaw) (Math|Rotator|BreakRotator _forward_rotation))
  (Variables|Turning|SetTurning true)
  (if (Variables|Turning|GetBackwards)
    (bind _turn_control (Timeline|Turn ReverseFromEnd)
      (:Update
        (Transformation|SetWorldRotation (Variables|Default|GetFirstPersonCamera) (Math|Rotator|Lerp(Rotator) _forward_rotation (Math|Rotator|MakeRotator _roll _pitch (+ _yaw (Math|Float|SelectFloat 180.1 179.9 Left))) _turn_control true) false false))
      (:Finished
        (Variables|Turning|SetTurning false)
        (Variables|Turning|SetBackwards (not (Variables|Turning|GetBackwards)))))
    (else
      (Timeline|Turn PlayFromStart))))

(event EventBeginPlay
  (bind _returnvalue (UserInterface|CreateWidget "/Game/Widgets/GUI_wg.GUI_wg_C"))
  (UserInterface|Viewport|AddtoViewport _returnvalue 0))

(fn ConstructionScript
  (Variables|Stamina|SetStamina (Variables|Stamina|GetMax%20Stamina))
  (Variables|Turning|SetForward%20Rotation (Transformation|GetWorldRotation (Variables|Default|GetFirstPersonCamera))))