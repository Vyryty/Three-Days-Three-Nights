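; Jesus actor that escapes the tomb and loses the game for the player if left uncovered for too long.
; Uncover starts a countdown of random length between the min and max escape times, and Cover pauses it.
; Once time runs out, escape waits until the cached PlayerGuard is not Backwards or is invalid.
; Escape reports the loss to the 3D3N game mode with message, tip and sound, then destroys the actor.
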(event Custom|Cover
  (Variables|Default|SetUncovered false))

(event Custom|Uncover
  (Variables|Default|SetUncovered true)
  (bind _output_get (Variables|Default|SetEscape%20Time (Math|Float|Lerp (Variables|Default|GetMin%20Escape%20Time) (Variables|Default|GetMax%20Escape%20Time) (Math|Random|RandomFloat))))
  (Variables|Default|SetEscape%20Timer _output_get))

(event Custom|Escape
  (bind _as3d3n_gm (Utilities|Casting|CastTo3D3N_gm (Game|GetGameMode))
    (:then
      (Default|Lose _as3d3n_gm "\"And when they looked, they saw that the stone was rolled away: for it was very great.\" - Mark 16:4 KJV" "Jesus Escaped" "Make sure to roll the stone back into place to keep Jesus in the tomb! It helps to have your assistant help you push the rock." "/Game/Audio/Sounds/Distorted_Hallelujah_Sound.Distorted_Hallelujah_Sound"))
    (:CastFailed
      _))
  (Actor|DestroyActor))

(event EventTick
  (params (DeltaSeconds :type Float%20%28single-precision%29))
  (if (Variables|Default|GetUncovered)
    (bind _output_get (Variables|Default|SetEscape%20Timer (- (Variables|Default|GetEscape%20Timer) DeltaSeconds)))
    (if (<= _output_get 0.0)
      (bind _player (Variables|Default|GetPlayer)
        (:then
          (if (not (Variables|/Game/Blueprints/PlayerGuard_bp.PlayerGuard_bp_C|GetBackwards _player))
            (CallFunction|Escape :!label _label)))
        (:else
          (goto _label))))))

(event EventBeginPlay
  (bind _outactors (Actor|GetAllActorsOfClass "/Game/Blueprints/PlayerGuard_bp.PlayerGuard_bp_C"))
  (Variables|Default|SetPlayer (Utilities|Array|Get(acopy) _outactors)))

(fn ConstructionScript)