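; Stone Blueprint that rolls between a start and end transform, which an external Push can drive back.
; On BeginPlay it scales roll speed, bonus delay and random wait by the game instance's Difficulty.
; Each Tick, pushing lowers Progress and resets the delay timer at zero; otherwise the stone rolls forward once the timer expires.
; Progress then lerps the mesh's relative location and rotation.
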(event Custom|Push
  (params (Extra%20Force :type Float%20%28double-precision%29))
  (Variables|NormalMovement|SetPushing true)
  (Variables|VariableMovement|SetForce Extra%20Force))

(event Custom|Stop%20Pushing
  (Variables|NormalMovement|SetPushing false)
  (Variables|VariableMovement|SetForce 0.0))

(event EventTick
  (params (DeltaSeconds :type Float%20%28single-precision%29))
  (Utilities|FlowControl|Sequence
    (:then_0
      (if (and (Variables|NormalMovement|GetPushing) (> (Variables|VariableMovement|GetForce) 0.0))
        (bind _output_get (Variables|NormalMovement|SetProgress (Math|Float|Clamp(Float) (- (Variables|NormalMovement|GetProgress) (* (Variables|VariableMovement|GetForce) DeltaSeconds)))))
        (if (<= _output_get 0.0)
          (Variables|NormalMovement|SetBonus%20Timer (+ (Variables|VariableMovement|GetBonus%20Time) (Math|Random|RandomFloatinRange 0.0 (Variables|VariableMovement|GetMax%20Wait%20Time)))))
        (elif (> (Variables|NormalMovement|GetBonus%20Timer) 0.0)
          (Variables|NormalMovement|SetBonus%20Timer (- (Variables|NormalMovement|GetBonus%20Timer) DeltaSeconds))
          (else
            (Variables|NormalMovement|SetProgress (Math|Float|Clamp(Float) (+ (Variables|NormalMovement|GetProgress) (* (Variables|VariableMovement|GetRoll%20Speed) DeltaSeconds))))))))
    (:then_1
      (Transformation|SetRelativeLocationAndRotation (Variables|Default|GetStaticMesh) (Math|Vector|Lerp(Vector) (Variables|NormalMovement|GetStarting%20Position) (Variables|NormalMovement|GetEnding%20Position) (Variables|NormalMovement|GetProgress)) (Math|Rotator|Lerp(Rotator) (Variables|NormalMovement|GetStarting%20Rotation) (Variables|NormalMovement|GetEnding%20Rotation) (Variables|NormalMovement|GetProgress) true) false false))))

(event EventBeginPlay
  (bind _as3d3n_gi (Utilities|Casting|CastTo3D3N_gi (Game|GetGameInstance)))
  (Variables|VariableMovement|SetRoll%20Speed (Math|Float|Lerp (Variables|NormalMovement|GetMin%20Roll%20Speed) (Variables|NormalMovement|GetMax%20Roll%20Speed) (/ (Math|Conversions|ToFloat(Integer) (Variables|/Game/Blueprints/3D3N_gi.3D3N_gi_C|GetDifficulty _as3d3n_gi)) (Variables|/Game/Blueprints/3D3N_gi.3D3N_gi_C|GetMax%20Difficulty _as3d3n_gi))))
  (bind _output_get (Variables|VariableMovement|SetBonus%20Time (Math|Float|Lerp (Variables|NormalMovement|GetMax%20Bonus%20Time) (Variables|NormalMovement|GetMin%20Bonus%20Time) (/ (Math|Conversions|ToFloat(Integer) (Variables|/Game/Blueprints/3D3N_gi.3D3N_gi_C|GetDifficulty _as3d3n_gi)) (Variables|/Game/Blueprints/3D3N_gi.3D3N_gi_C|GetMax%20Difficulty _as3d3n_gi)))))
  (bind _output_get_2 (Variables|VariableMovement|SetMax%20Wait%20Time (Math|Float|Lerp (Variables|NormalMovement|GetMax%20M%20Wait%20Time) (Variables|NormalMovement|GetMin%20M%20Wait%20Time) (/ (Math|Conversions|ToFloat(Integer) (Variables|/Game/Blueprints/3D3N_gi.3D3N_gi_C|GetDifficulty _as3d3n_gi)) (Variables|/Game/Blueprints/3D3N_gi.3D3N_gi_C|GetMax%20Difficulty _as3d3n_gi)))))
  (Variables|NormalMovement|SetBonus%20Timer (+ _output_get (Math|Random|RandomFloatinRange 0.0 _output_get_2))))

(fn ConstructionScript)