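; Game mode for a night-survival game that runs the clock, win and loss screens, and retry.
; Tick advances six hours over NightLength minutes and, when the Roman-numeral hour reads VI, swaps the guard player's GUI for a victory widget, with no guard against repeating.
; Lose stops the clock, plays a sound and shows a widget with message, reason and tip.
; Retry resets state and reopens the current level.
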(event Custom|Lose
  (params (Lose%20Message :type Text) (Lose%20Reason :type Text) (Lose%20Tip :type Text) (Lose%20Sound :type Sound%20Base%20Object%20Reference))
  (Utilities|FlowControl|Sequence
    (:then_0
      (Variables|Default|SetLost true))
    (:then_1
      (Utilities|IsValid Lose%20Sound
        (:Is%20Valid
          (Audio|PlaySoundatLocation Lose%20Sound "0, 0, 0" "0, 0, 0" 1.0 1.0 0.0 0 0 0 0))))
    (:then_2
      (bind _player (Variables|Default|GetPlayer)
        (:then
          (Widget|RemovefromParent (Variables|/Game/Blueprints/PlayerGuard_bp.PlayerGuard_bp_C|GetGUI _player))
          (bind _returnvalue (UserInterface|CreateWidget "/Game/Widgets/Lose_wg.Lose_wg_C"))
          (Variables|/Game/Widgets/Lose_wg.Lose_wg_C|SetLose%20Message _returnvalue Lose%20Message)
          (Variables|/Game/Widgets/Lose_wg.Lose_wg_C|SetLose%20Reason _returnvalue Lose%20Reason)
          (Variables|/Game/Widgets/Lose_wg.Lose_wg_C|SetLose%20Tip _returnvalue Lose%20Tip)
          (UserInterface|Viewport|AddtoViewport _returnvalue 0))
        (:else)))))

(event Custom|Retry
  (Variables|Default|SetLost false)
  (Variables|Default|SetTime 0.0)
  (bind _returnvalue (Game|GetCurrentLevelName true))
  (Game|OpenLevel(byName) (Utilities|String|StringToName _returnvalue)))

(event EventTick
  (params (DeltaSeconds :type Float%20%28single-precision%29))
  (if (not (Variables|Default|GetLost))
    (Variables|Default|SetTime (+ (Variables|Default|GetTime) (/ (* DeltaSeconds 6.0) (* (Variables|Default|GetNight%20Length) 6e+01))))
    (if (Utilities|Enum|Equal(Enum) (CallFunction|GetTimeNumeral) "VI")
      (bind _player (Variables|Default|GetPlayer)
        (:then
          (Widget|RemovefromParent (Variables|/Game/Blueprints/PlayerGuard_bp.PlayerGuard_bp_C|GetGUI _player))
          (bind _returnvalue (UserInterface|CreateWidget "/Game/Widgets/Victory_wg.Victory_wg_C"))
          (UserInterface|Viewport|AddtoViewport _returnvalue 0))
        (:else)))))

(event EventBeginPlay
  (Variables|Default|SetLost false)
  (bind _asplayer_guard_bp (Utilities|Casting|CastToPlayerGuard_bp (Game|GetPlayerCharacter 0)))
  (Variables|Default|SetPlayer _asplayer_guard_bp))

(fn ConstructionScript)

(fn GetTimeNumeral
  (bind _numerals (LocalVariables|GetNumerals))
  (return (Utilities|Array|Get(acopy) _numerals (Math|Integer|Clamp(Integer) (Math|Float|Truncate (Variables|Default|GetTime)) 0 (Utilities|Array|Length _numerals)))))