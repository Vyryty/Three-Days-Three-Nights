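; Fire actor that drives a point light and a Niagara effect from a single Strength value.
; Each tick it clamps Strength between zero and one, then scales light intensity by its square and the "Fire Strength" particle parameter linearly, so the light dims faster than the flames.
; The construction script initializes both light and effect at their configured maximums, independent of Strength.
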(event EventTick
  (params (DeltaSeconds :type Float%20%28single-precision%29))
  (bind _output_get (Variables|Default|SetStrength (Math|Float|Clamp(Float) (Variables|Default|GetStrength))))
  (Rendering|Components|Light|SetIntensity (Variables|Default|GetPointLight) (Math|Float|Lerp 0.0 (Variables|Default|GetMax%20Brightness) (* _output_get _output_get)))
  (Effects|Components|ParticleSystem|SetFloatParameter (Variables|Default|GetNiagara) "Fire Strength" (Math|Float|Lerp 0.0 (Variables|Default|GetMax%20Strength) _output_get)))

(fn ConstructionScript
  (Rendering|Components|Light|SetIntensity (Variables|Default|GetPointLight) (Variables|Default|GetMax%20Brightness))
  (Effects|Components|ParticleSystem|SetFloatParameter (Variables|Default|GetNiagara) "Fire Strength" (Variables|Default|GetMax%20Strength)))