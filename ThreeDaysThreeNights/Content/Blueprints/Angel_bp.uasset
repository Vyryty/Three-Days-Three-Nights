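; Angel is a hazard that periodically moves into the forest to hunt the assistant guard.
; A looping timeline moves it between its original and hunting positions with audio, using random linger times and a difficulty-scaled, randomized wait.
; While it lingers and the assistant is away from camp, a random pounce countdown runs on Tick, then defeats the assistant and destroys Angel.
; The game mode's Done flag blocks pouncing and silences the audio.
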(event EventBeginPlay
  (bind _audio (Variables|Default|GetAudio))
  (bind _outactors (Actor|GetAllActorsOfClass "/Game/Blueprints/AssistantGuard_bp.AssistantGuard_bp_C"))
  (Variables|Default|SetAssistant (Utilities|Array|Get(acopy) _outactors))
  (bind _as3d3n_gm (Utilities|Casting|CastTo3D3N_gm (Game|GetGameMode)))
  (bind _as3d3n_gi (Utilities|Casting|CastTo3D3N_gi (Game|GetGameInstance)))
  (if (not (Variables|/Game/Blueprints/3D3N_gm.3D3N_gm_C|GetDone _as3d3n_gm))
    (Utilities|FlowControl|Delay (+ (Math|Float|Lerp (Variables|Hunting|GetMin%20Wait%20Time) (Variables|Hunting|GetMax%20Wait%20Time) (/ (Variables|/Game/Blueprints/3D3N_gi.3D3N_gi_C|GetDifficulty _as3d3n_gi) (Math|Conversions|ToFloat(Integer) (Variables|/Game/Blueprints/3D3N_gi.3D3N_gi_C|GetMax%20Difficulty _as3d3n_gi)))) (Math|Random|RandomFloatinRange 0.0 (Variables|Hunting|GetMax%20Random%20Wait%20Time))) :!label _label)
    (Audio|Components|Audio|Play _audio 0.0)
    (bind (_direction _position_control) (Timeline|Position Play)
      (:Update
        (Transformation|SetWorldLocation (Variables|Default|GetAngel) (Math|Vector|Lerp(Vector) (Variables|Default|GetOriginal%20Position) (Variables|Default|GetHunting%20Position) _position_control) false false))
      (:Finished
        (Audio|Components|Audio|Stop _audio)
        (if (== _direction 0)
          (Variables|Hunting|SetIn%20Forest true)
          (Utilities|FlowControl|Delay (Math|Random|RandomFloatinRange (Variables|Hunting|GetMin%20Linger%20Time) (Variables|Hunting|GetMax%20Linger%20Time)))
          (Variables|Hunting|SetIn%20Forest false)
          (Audio|Components|Audio|Play _audio 0.0)
          (Timeline|Position Reverse)
          (else
            (goto _label)))))))

(event EventTick
  (params (DeltaSeconds :type Float%20%28single-precision%29))
  (bind _as3d3n_gm (Utilities|Casting|CastTo3D3N_gm (Game|GetGameMode)))
  (bind _assistant (Variables|Default|GetAssistant)
    (:then
      (Utilities|FlowControl|Sequence
        (:then_0
          (if (Math|Boolean|ANDBoolean (Variables|Hunting|GetIn%20Forest) (not (Variables|/Game/Blueprints/AssistantGuard_bp.AssistantGuard_bp_C|GetAt%20Camp _assistant)) (not (Variables|/Game/Blueprints/3D3N_gm.3D3N_gm_C|GetDone _as3d3n_gm)))
            (if (<= (Variables|Hunting|GetPounce%20Timer) 0.0)
              (Default|Defeat (Variables|Default|GetAssistant))
              (Actor|DestroyActor)
              (else
                (Variables|Hunting|SetPounce%20Timer (- (Variables|Hunting|GetPounce%20Timer) DeltaSeconds))))
            (else
              (Variables|Hunting|SetPounce%20Timer (Math|Random|RandomFloatinRange 0.0 (Variables|Hunting|GetMax%20Pounce%20Time))))))
        (:then_1
          (if (Variables|/Game/Blueprints/3D3N_gm.3D3N_gm_C|GetDone _as3d3n_gm)
            (Audio|Components|Audio|Stop (Variables|Default|GetAudio))))))
    (:else)))

(fn ConstructionScript
  (Variables|Default|SetOriginal%20Position (Transformation|GetWorldLocation (Variables|Default|GetAngel))))