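; Guard troupe that patrols out and back along control points, pausing between round trips for timed visits announced by hello and goodbye sounds.
; BeginPlay derives visit frequency from game difficulty and trip duration from night length.
; Until the game mode is Done, Tick moves the Leader at constant speed by mapping elapsed time to path distance, using mirrored indices for the return leg.
; IsClose flags each trip's first and last tenth.
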(event Custom|Restart%20Movement
  (Variables|Interpolation|SetControl%20Time 0.0)
  (Variables|Interpolation|SetCurrent%20Point 0)
  (Variables|Interpolation|SetPlaying true)
  (Variables|Visiting|SetVisiting false)
  (Audio|PlaySoundatLocation "/Game/Audio/Sounds/Goodbye.Goodbye" (Transformation|GetWorldLocation (Variables|Default|GetLeader)) "0, 0, 0" 1.0 1.0 0.0 0 0 0 0))

(event EventBeginPlay
  (bind _min_visit_frequency (Variables|Visiting|GetMin%20Visit%20Frequency))
  (Utilities|FlowControl|Sequence
    (:then_0
      (bind _as3d3n_gi (Utilities|Casting|CastTo3D3N_gi (Game|GetGameInstance))
        (:then
          (Variables|Visiting|SetVisit%20Frequency (Math|Float|Round (+ (* (/ (Variables|/Game/Blueprints/3D3N_gi.3D3N_gi_C|GetDifficulty _as3d3n_gi) (Math|Conversions|ToFloat(Integer) (Variables|/Game/Blueprints/3D3N_gi.3D3N_gi_C|GetMax%20Difficulty _as3d3n_gi))) (- (Variables|Visiting|GetMax%20Visit%20Frequency) _min_visit_frequency)) _min_visit_frequency))))
        (:CastFailed
          (Variables|Visiting|SetVisit%20Frequency 2))))
    (:then_1
      (bind _as3d3n_gm (Utilities|Casting|CastTo3D3N_gm (Game|GetGameMode))
        (:then
          (Variables|Interpolation|SetDuration (- (/ (* (Variables|/Game/Blueprints/3D3N_gm.3D3N_gm_C|GetNight%20Length _as3d3n_gm) 6e+01) (Variables|Visiting|GetVisit%20Frequency)) (Variables|Visiting|GetVisit%20Time))))
        (:CastFailed
          (Variables|Interpolation|SetDuration 15.0))))
    (:then_2
      (Variables|Interpolation|SetTotal%20Distance (* (CallFunction|CalculateTotalDistance (Variables|Interpolation|GetControl%20Points)) 2.0))
      (CallFunction|RestartMovement))))

(event EventTick
  (params (DeltaSeconds :type Float%20%28single-precision%29))
  (bind _as3d3n_gm (Utilities|Casting|CastTo3D3N_gm (Game|GetGameMode)))
  (if (not (Variables|/Game/Blueprints/3D3N_gm.3D3N_gm_C|GetDone _as3d3n_gm))
    (CallFunction|Interpolate DeltaSeconds)
    (if (and (not (Variables|Interpolation|GetPlaying)) (not (Variables|Visiting|GetVisiting)))
      (Variables|Visiting|SetVisiting true)
      (Audio|PlaySoundatLocation "/Game/Audio/Sounds/Hello.Hello" (Transformation|GetWorldLocation (Variables|Default|GetLeader)) "0, 0, 0" 1.0 1.0 0.0 0 0 0 0)
      (Utilities|FlowControl|Delay (Variables|Visiting|GetVisit%20Time))
      (CallFunction|RestartMovement))))

(fn ConstructionScript
  (bind _output_get (Variables|Interpolation|SetOriginal%20Position (Transformation|GetWorldLocation (Variables|Default|GetLeader))))
  (Variables|Interpolation|SetPrevious%20Position _output_get))

(fn Interpolate
  (params (Delta%20Seconds :type Float%20%28double-precision%29))
  (bind _control_points (Variables|Interpolation|GetControl%20Points))
  (bind _current_point (Variables|Interpolation|GetCurrent%20Point))
  (bind _control_points_2 (Variables|Interpolation|GetControl%20Points))
  (bind _current_point_2 (Variables|Interpolation|GetCurrent%20Point))
  (bind _duration (Variables|Interpolation|GetDuration))
  (bind _element (CallFunction|GetBouncingIndex _control_points _current_point))
  (bind _element_2 (CallFunction|GetBouncingIndex _control_points_2 _current_point_2))
  (bind _returnvalue (+ _current_point 1))
  (bind _returnvalue_2 (+ _current_point_2 1))
  (bind _element_3 (CallFunction|GetBouncingIndex _control_points _returnvalue))
  (bind _element_4 (CallFunction|GetBouncingIndex _control_points_2 _returnvalue_2))
  (bind _returnvalue_3 (Math|Vector|Distance(Vector) _element _element_3))
  (if (Variables|Interpolation|GetPlaying)
    (bind _output_get (Variables|Interpolation|SetControl%20Time (Math|Float|Clamp(Float) (+ (Variables|Interpolation|GetControl%20Time) Delta%20Seconds) 0.0 _duration)))
    (Variables|Interpolation|SetCurrent%20Distance (Math|Float|Lerp 0.0 (Variables|Interpolation|GetTotal%20Distance) (/ _output_get _duration)))
    (Variables|Interpolation|SetDirection (* (/ (Variables|Interpolation|GetTotal%20Distance) (Variables|Interpolation|GetDuration)) (Math|Float|SelectFloat 1.0 -1.0 (< (Variables|Interpolation|GetControl%20Time) (* (Variables|Interpolation|GetDuration) 0.5)))))
    (bind _output_get_2 (LocalVariables|SetSnapped%20Total%20Distance (CallFunction|CalculateTotalDistance (CallFunction|GatherPoints (Variables|Interpolation|GetCurrent%20Point)))))
    (bind _output_get_3 (LocalVariables|SetAB%20Distance (- (Variables|Interpolation|GetCurrent%20Distance) _output_get_2)))
    (Utilities|FlowControl|Sequence
      (:then_0
        (if (>= (- _output_get_3 _returnvalue_3) -0.0001)
          (Math|Integer|IncrementInt (Variables|Interpolation|GetCurrent%20Point)
            (:%20%20
              (LocalVariables|SetSnapped%20Total%20Distance (+ (LocalVariables|GetSnapped%20Total%20Distance) _returnvalue_3))
              (LocalVariables|SetAB%20Distance (- (LocalVariables|GetAB%20Distance) _returnvalue_3))))))
      (:then_1
        (if (>= (Variables|Interpolation|GetCurrent%20Point) (- (* (Utilities|Array|Length _control_points_2) 2) 2))
          (Variables|Interpolation|SetPlaying false)
          (else
            (Transformation|SetWorldLocation (Variables|Default|GetLeader) (+ (Variables|Interpolation|GetOriginal%20Position) (Math|Vector|MakeVector (* (.x (Math|Vector|Lerp(Vector) _element_2 _element_4 (/ (LocalVariables|GetAB%20Distance) (Math|Vector|Distance(Vector) _element_2 _element_4)))) -0.75) (* (.y (Math|Vector|Lerp(Vector) _element_2 _element_4 (/ (LocalVariables|GetAB%20Distance) (Math|Vector|Distance(Vector) _element_2 _element_4)))) -0.75) (.z (Math|Vector|Lerp(Vector) _element_2 _element_4 (/ (LocalVariables|GetAB%20Distance) (Math|Vector|Distance(Vector) _element_2 _element_4)))))) false false)))))))

(fn CalculateTotalDistance
  (params (Control%20Points :type Array%20of%20Vectors))
  (for _array_element Control%20Points
    (if (LocalVariables|GetInitial%20Set)
      (LocalVariables|SetDist (+ (LocalVariables|GetDist) (Math|Vector|Distance(Vector) (LocalVariables|GetPoint%20A) _array_element)))
      (else
        (LocalVariables|SetInitial%20Set true)))
    (LocalVariables|SetPoint%20A _array_element))
  (return (LocalVariables|GetDist)))

(fn IsClose
  (bind _control_time (Variables|Interpolation|GetControl%20Time))
  (bind _duration (Variables|Interpolation|GetDuration))
  (bind _returnvalue (/ _control_time _duration))
  (return (or (< _returnvalue 0.1) (> _returnvalue 0.9))))

(fn GatherPoints
  (params (Bouncing%20Index :type Integer))
  (bind _points (LocalVariables|GetPoints))
  (for _index (range 0 Bouncing%20Index)
    (Utilities|Array|Add _points (CallFunction|GetBouncingIndex (Variables|Interpolation|GetControl%20Points) _index)))
  (return _points))

(fn GetBouncingIndex
  (params (Array :type Array%20of%20Vectors) (Index :type Integer))
  (bind _returnvalue (Utilities|Array|Length Array))
  (return (Utilities|Array|Get(acopy) Array (Math|Integer|SelectInt Index (Utilities|Operators|Subtract _returnvalue (- (+ Index 1) _returnvalue) 1) (< Index _returnvalue)))))